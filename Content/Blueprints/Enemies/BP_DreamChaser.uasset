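; BP_DreamChaser is an enemy that carries a looping smoke-monster wind sound and reacts to breaking corridor lights.
; BeginPlay attaches the sound and binds OnLightBreaking, which plays a random bulb-pop at the light's position; Tick restarts the sound whenever it stops.
; Capsule overlaps give tagged corridor light meshes dynamic materials and store them.
; The emissive shutoff is unconnected, leaving Tick's loop over those materials empty.
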(event `self.ReceiveBeginPlay`
  (bind _returnvalue (`GameplayStatics.SpawnSoundAttached` "/Game/Assets/Sounds/SmokeCreature/GRIEF_SMOKE.GRIEF_SMOKE" (`self.SoundAttachment`) "None" (0.0 0.0 0.0) (struct) "KeepRelativeOffset" false 1.0 1.0 0.0 "/Game/Assets/Sounds/AttenuationSettings/AS_SmokeMonster_Wind.AS_SmokeMonster_Wind" null false))
  (set `self.EnemySound` _returnvalue)
  (add `self.OnLightBreaking` (delegate `OnLightBreaking_Event_0`)))

(event `OnLightBreaking_Event_0` :!signature `self.OnLightBreaking`
  (params (LightPosition :type "Vector Structure"))
  (`GameplayStatics.PlaySoundAtLocation` (`KismetArrayLibrary.Array_Random` (`|MakeArray` "/Game/Assets/Sounds/Environment/LightbulbExplode/Lightbulb_Explode_1.Lightbulb_Explode_1" "/Game/Assets/Sounds/Environment/LightbulbExplode/Lightbulb_Explode_2.Lightbulb_Explode_2" "/Game/Assets/Sounds/Environment/LightbulbExplode/Lightbulb_Explode_3.Lightbulb_Explode_3" :!type "SoundBase Object Reference")) LightPosition (struct) 0.2 1.0 0.0 "/Game/Assets/Sounds/AttenuationSettings/AS_SmokeMonster_LightBulbPop.AS_SmokeMonster_LightBulbPop" null null))

(event `self.ReceiveTick`
  (params (DeltaSeconds :type "Float (single-precision)"))
  (if (not (`AudioComponent.IsPlaying` (`self.EnemySound`)))
    (`AudioComponent.Play` (`self.EnemySound`) 0.0)
    (for _array_element (`self.LightMeshMaterialInstances`)
      _)))

(event `self.Capsule.OnComponentBeginOverlap`
  (params (OverlappedComponent :type "PrimitiveComponent Object Reference") (OtherActor :type "Actor Object Reference") (OtherComp :type "PrimitiveComponent Object Reference") (OtherBodyIndex :type Integer) (bFromSweep :type Boolean) (SweepResult :type "HitResult Structure (by ref)"))
  (bind _asstatic_mesh_component (cast `StaticMeshComponent` OtherComp))
  (if (`ActorComponent.ComponentHasTag` _asstatic_mesh_component "CorridorLightMesh")
    (bind _returnvalue (`PrimitiveComponent.CreateDynamicMaterialInstance` _asstatic_mesh_component 0 "/Game/Assets/Materials/MaterialInstances/MI_Light_02.MI_Light_02" "None"))
    (`KismetArrayLibrary.Array_Add` (`self.LightMeshMaterialInstances`) _returnvalue)))

(fn `UserConstructionScript`)