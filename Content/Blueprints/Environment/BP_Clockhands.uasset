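; Clock hands actor that acts as a move-limited countdown to the player's death.
; Each MoveDemHands call steps the minute hand by a fixed rotation, plays a winding sound and increments a counter.
; On the sixth move it also plays a fade-out level sequence, whose finish callback flags HasDied on the game instance and opens the Anger environment level.
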(event `self.MoveDemHands`
  (`SceneComponent.K2_AddLocalRotation` (`self.MinuteHand`) (struct :`Roll` -30.0) false false)
  (bind _output_get (set `self.HandMoves` (+ (`self.HandMoves`) 1)))
  (if (>= _output_get 6)
    (`GameplayStatics.PlaySoundAtLocation` "/Game/Assets/Sounds/Clock/Clock_Winding.Clock_Winding" (`self.K2_GetActorLocation`) (struct) 1.0 1.0 0.0 null null null)
    (bind (_outactor _returnvalue) (`LevelSequencePlayer.CreateLevelSequencePlayer` (`self.FadeOutSequence`) (make `MovieSceneSequencePlaybackSettings` true)))
    (add `MovieSceneSequencePlayer.OnFinished` _returnvalue (delegate `On Finished Sequence`))
    (else
      (`GameplayStatics.PlaySoundAtLocation` "/Game/Assets/Sounds/Clock/Clock_Winding.Clock_Winding" (`self.K2_GetActorLocation`) (struct) 1.0 1.0 0.0 null null null))))

(event `On Finished Sequence`
  (bind _asbp_game_instance (cast `/Game/Blueprints/System/BP_GameInstance` (`GameplayStatics.GetGameInstance`)))
  (set `/Game/Blueprints/System/BP_GameInstance.HasDied` true _asbp_game_instance)
  (`GameplayStatics.OpenLevelBySoftObjectPtr` "/Game/Levels/TestLevels/SamuelLevels/L_Anger_Environment.L_Anger_Environment"))

(fn `UserConstructionScript`)