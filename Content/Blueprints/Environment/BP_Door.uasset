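; BP_Door is a door Blueprint that supplies audio and UI feedback for door interactions.
; Interact events for open, close, locked and key-locked play a sound at the door's location, with both locked cases sharing one sound.
; The key-locked event also shows a locked-door widget briefly, using a flag to prevent duplicate widgets while the delay runs.
; It contains no door movement or lock logic, only responses to these events.
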(event `self.ReceiveBeginPlay`)

(event `self.OnLockedDoorInteract`
  (`GameplayStatics.PlaySoundAtLocation` "/Game/Assets/Sounds/131028__dymewiz__locking-a-door-03.131028__dymewiz__locking-a-door-03" (`self.K2_GetActorLocation`) (struct) 1.0 1.0 0.0 null null null))

(event `self.OnOpenDoorInteract`
  (`GameplayStatics.PlaySoundAtLocation` "/Game/Assets/Sounds/Door/Door_Opening.Door_Opening" (`self.K2_GetActorLocation`) (struct) 1.0 1.0 0.0 null null null))

(event `self.OnCloseDoorInteract`
  (`GameplayStatics.PlaySoundAtLocation` "/Game/Assets/Sounds/Door/Door_Close.Door_Close" (`self.K2_GetActorLocation`) (struct) 1.0 1.0 0.0 null null null))

(event `self.OnKeyLockedDoorInteract`
  (`GameplayStatics.PlaySoundAtLocation` "/Game/Assets/Sounds/131028__dymewiz__locking-a-door-03.131028__dymewiz__locking-a-door-03" (`self.K2_GetActorLocation`) (struct) 1.0 1.0 0.0 null null null)
  (if (not (`self.bIsShowingLockedUI`))
    (set `self.bIsShowingLockedUI` true)
    (bind _returnvalue (`|CreateWidget` "/Game/Blueprints/Widgets/WBP_LockedDoorInteract.WBP_LockedDoorInteract_C"))
    (`UserWidget.AddToViewport` _returnvalue 0)
    (`KismetSystemLibrary.Delay` 2.0)
    (`Widget.RemoveFromParent` _returnvalue)
    (set `self.bIsShowingLockedUI` false)))

(fn `UserConstructionScript`)