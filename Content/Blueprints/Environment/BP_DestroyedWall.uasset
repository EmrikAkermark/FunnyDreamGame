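; BP_DestroyedWall is a short-lived wall debris actor that bursts apart and dissolves once spawned.
; On BeginPlay it applies a radial impulse to nearby overlapped components from an origin offset along its negative right vector, compensating for a rotated actor.
; It gives its static meshes dynamic dissolve materials, and Tick drives their DissolveT parameter with elapsed time.
; A short delay then destroys the actor.
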(event `self.ReceiveBeginPlay`
  (bind _outcomponents (`KismetSystemLibrary.SphereOverlapComponents` (`self.K2_GetActorLocation`) 300.0 (`self.Object Types`) "/Script/Engine.PrimitiveComponent"))
  (`PrimitiveComponent.AddRadialImpulse` _outcomponents (+ (`self.K2_GetActorLocation`) (* (`KismetMathLibrary.NegateVector` (`self.GetActorRightVector`)) 1500.0)) 5000.0 5000.0 "RIF_Linear" false)
  (for _array_element (`self.K2_GetComponentsByClass` "/Script/Engine.StaticMeshComponent")
    (bind _returnvalue (`PrimitiveComponent.CreateDynamicMaterialInstance` _array_element 0 "/Game/Assets/ParticleSystems/Materials/MaterialInstances/PMI_DissolvingCel.PMI_DissolvingCel" "None"))
    (`KismetArrayLibrary.Array_Add` (`self.MaterialInstances`) _returnvalue)
    (set `self.DissolveT` 0.0)
    (`KismetSystemLibrary.Delay` 1.5)
    (`self.K2_DestroyActor`)))

(event `self.ReceiveTick`
  (params (DeltaSeconds :type "Float (single-precision)"))
  (set `self.DissolveT` (+ DeltaSeconds (`self.DissolveT`)))
  (for _array_element (`self.MaterialInstances`)
    (`MaterialInstanceDynamic.SetScalarParameterValue` _array_element "DissolveT" (`self.DissolveT`))))

(fn `UserConstructionScript`)