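; A trigger volume that switches a referenced actor on or off when the player enters it.
; On BeginPlay it applies StartState to both the visibility and collision of ActorToToggle.
; When a PlayerPawn begins overlapping the Box, it applies StateToSwitchTo the same way.
; The switch sets a fixed state rather than alternating, and nothing reverts it when the overlap ends.
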(event `self.ReceiveBeginPlay`
  (bind _actortotoggle (`self.ActorToToggle`))
  (bind _startstate (`self.StartState`))
  (`self.SetActorHiddenInGame` _actortotoggle (not _startstate))
  (`self.SetActorEnableCollision` _actortotoggle _startstate))

(event `self.Box.OnComponentBeginOverlap`
  (params (OverlappedComponent :type "PrimitiveComponent Object Reference") (OtherActor :type "Actor Object Reference") (OtherComp :type "PrimitiveComponent Object Reference") (OtherBodyIndex :type Integer) (bFromSweep :type Boolean) (SweepResult :type "HitResult Structure (by ref)"))
  (bind _actortotoggle (`self.ActorToToggle`))
  (bind _statetoswitchto (`self.StateToSwitchTo`))
  (cast `PlayerPawn` OtherActor)
  (`self.SetActorHiddenInGame` _actortotoggle (not _statetoswitchto))
  (`self.SetActorEnableCollision` _actortotoggle _statetoswitchto))

(fn `UserConstructionScript`)