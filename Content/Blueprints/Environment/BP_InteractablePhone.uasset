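; Interactable phone prop that rings in the world and starts a dialog when the player interacts with it.
; On BeginPlay it pre-spawns a stopped, attenuated sound component at its location, then plays it after a short delay unless the phone has already been activated.
; OnInteract triggers the DialogSystem, flags the phone as activated, destroys the sound and hides the phone mesh.
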(event `self.ReceiveBeginPlay`
  (bind _returnvalue (`GameplayStatics.SpawnSoundAtLocation` "/Game/Assets/Sounds/COMTelph_Dial_phone__ID_0001__BSB.COMTelph_Dial_phone__ID_0001__BSB" (`self.K2_GetActorLocation`) (struct) 0.5 1.0 0.0 "/Game/Assets/Sounds/AttenuationSettings/AS_MobilePhone_Ring.AS_MobilePhone_Ring" null false))
  (bind _output_get (set `self.SoundComponent` _returnvalue))
  (`AudioComponent.Stop` _output_get)
  (`KismetSystemLibrary.Delay` 5.0)
  (if (not (`self.PhoneActivated`))
    (`AudioComponent.Play` (`self.SoundComponent`) 0.0)))

(event `self.OnInteract`
  (params (Interacter :type "FGInteractionComponent Object Reference"))
  (bind _soundcomponent (`self.SoundComponent`))
  (`/Game/Blueprints/System/BP_DialogSystem.StartDialog` (`self.DialogSystem`))
  (set `self.PhoneActivated` true)
  (`AudioComponent.Stop` _soundcomponent)
  (`ActorComponent.K2_DestroyComponent` _soundcomponent)
  (`SceneComponent.SetVisibility` (`self.PhoneMesh`) false false))

(fn `UserConstructionScript`)