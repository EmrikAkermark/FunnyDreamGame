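; Level intro actor that plays an opening transition when a level begins.
; In the office level it auto-plays a wake-up sequence.
; Elsewhere it checks the game instance's death flag, playing a fade-from-black sequence after a death or otherwise a fade widget showing the level name image.
; Sequence actors and the widget are removed when they finish.
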(event `OfficeAwake`
  (`self.K2_DestroyActor` (stale `self.ReceiveBeginPlay` _outactor)))

(event `IntroFinish`
  (`self.K2_DestroyActor` (stale `self.ReceiveBeginPlay` _outactor_2)))

(event `self.ReceiveBeginPlay`
  (bind _moviescenesequenceplaybacksettings (make `MovieSceneSequencePlaybackSettings` true))
  (bind _returnvalue (`GameplayStatics.GetCurrentLevelName` true))
  (if (`KismetStringLibrary.EqualEqual_StrStr` _returnvalue "L_Amelie_OfficeEnviroment")
    (bind (_outactor _returnvalue_2) (`LevelSequencePlayer.CreateLevelSequencePlayer` "/Game/Cinematics/OfficeWake.OfficeWake" _moviescenesequenceplaybacksettings))
    (add `MovieSceneSequencePlayer.OnFinished` _returnvalue_2 (delegate `OfficeAwake`))
    (else
      (bind _asbp_game_instance (cast `/Game/Blueprints/System/BP_GameInstance` (`GameplayStatics.GetGameInstance`))
        (:`then`
          (bind _newparam (`/Game/Blueprints/System/BP_GameInstance.GetHasDied` _asbp_game_instance))
          (if _newparam
            (bind (_outactor_2 _returnvalue_3) (`LevelSequencePlayer.CreateLevelSequencePlayer` "/Game/Cinematics/FadeFromBlack.FadeFromBlack" _moviescenesequenceplaybacksettings))
            (add `MovieSceneSequencePlayer.OnFinished` _returnvalue_3 (delegate `IntroFinish`))
            (else
              (bind _returnvalue_4 (`|CreateWidget` "/Game/Blueprints/Widgets/FadeWithText.FadeWithText_C"))
              (`UserWidget.AddToViewport` _returnvalue_4 0)
              (bind _astexture_2d (cast `Texture2D` (`self.LevelNameImage`)))
              (`Image.SetBrushFromTexture` (`/Game/Blueprints/Widgets/FadeWithText.LevelName` _returnvalue_4) _astexture_2d true)
              (`|PlayAnimationTimeRange` _returnvalue_4 (`/Game/Blueprints/Widgets/FadeWithText.TextFade` _returnvalue_4)
                (:`Finished`
                  (`Widget.RemoveFromParent` _returnvalue_4))))))
        (:`CastFailed`
          (`KismetSystemLibrary.PrintString` "OOps"))))))

(fn `UserConstructionScript`)