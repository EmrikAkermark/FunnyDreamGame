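; Player pawn Blueprint that handles being caught by a DreamChaser and plays footstep audio.
; Overlapping a DreamChaser actor plays the PlayerDeathFadeToBlack level sequence.
; When the sequence finishes, it sets HasDied on BP_GameInstance and calls RestartLevelOnDeath.
; The movement component's OnStepTaken event plays a random one of eight footstep sounds at the Feet component's location.
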(event `On Finished Sequence`
  (bind _asbp_game_instance (cast `/Game/Blueprints/System/BP_GameInstance` (`GameplayStatics.GetGameInstance`)))
  (set `/Game/Blueprints/System/BP_GameInstance.HasDied` true _asbp_game_instance)
  (`self.RestartLevelOnDeath`))

(event `self.ReceiveActorBeginOverlap`
  (params (OtherActor :type "Actor Object Reference"))
  (if (`KismetMathLibrary.ClassIsChildOf` (`GameplayStatics.GetObjectClass` OtherActor) "/Script/FunnyDreamGame.DreamChaser")
    (bind (_outactor _returnvalue) (`LevelSequencePlayer.CreateLevelSequencePlayer` "/Game/Cinematics/PlayerDeathFadeToBlack.PlayerDeathFadeToBlack" (make `MovieSceneSequencePlaybackSettings` true)))
    (add `MovieSceneSequencePlayer.OnFinished` _returnvalue (delegate `On Finished Sequence`))))

(event `self.MovementComponent.OnStepTaken`
  (`GameplayStatics.PlaySoundAtLocation` (`KismetArrayLibrary.Array_Random` (`|MakeArray` "/Game/Assets/Sounds/Footsteps/SyncedFootsteps/Synced_Footstep_1.Synced_Footstep_1" "/Game/Assets/Sounds/Footsteps/SyncedFootsteps/Synced_Footstep_2.Synced_Footstep_2" "/Game/Assets/Sounds/Footsteps/SyncedFootsteps/Synced_Footstep_3.Synced_Footstep_3" "/Game/Assets/Sounds/Footsteps/SyncedFootsteps/Synced_Footstep_4.Synced_Footstep_4" "/Game/Assets/Sounds/Footsteps/SyncedFootsteps/Synced_Footstep_5.Synced_Footstep_5" "/Game/Assets/Sounds/Footsteps/SyncedFootsteps/Synced_Footstep_6.Synced_Footstep_6" "/Game/Assets/Sounds/Footsteps/SyncedFootsteps/Synced_Footstep_7.Synced_Footstep_7" "/Game/Assets/Sounds/Footsteps/SyncedFootsteps/Synced_Footstep_8.Synced_Footstep_8" :!type "SoundBase Object Reference")) (`SceneComponent.K2_GetComponentLocation` (`self.Feet`)) (struct) 0.2 1.0 0.0 null null null))

(fn `UserConstructionScript`)