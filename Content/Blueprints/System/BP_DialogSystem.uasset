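; BP_DialogSystem runs a dialogue sequence on screen, then triggers a level load through BP_LevelSelector when it ends.
; StartDialog, guarded against repeat calls, creates WBP_DialogueUI and binds to the player pawn's next and previous input dispatchers.
; Those inputs progress or regress the dialogue, and change events refresh the widget's text and portrait.
; On dialogue end, it calls LoadLevel and removes the dialogue widgets.
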(event `StartDialog`
  (if (not (`self.IsDialogRunning`))
    (set `self.IsDialogRunning` true)
    (add `self.OnDialogChanged` (delegate `OnDialogChanged_Event_0`))
    (bind _returnvalue (`|CreateWidget` "/Game/Blueprints/Widgets/WBP_DialogueUI.WBP_DialogueUI_C"))
    (bind _output_get (set `self.DialogBox` _returnvalue))
    (`UserWidget.AddToViewport` _output_get 0)
    (`self.UpdateDialog`)
    (bind _asbp_player_pawn (cast `/Game/Blueprints/PlayerPawns/BP_PlayerPawn` (`GameplayStatics.GetPlayerPawn` 0))
      (:`then`
        (add `PlayerPawn.DialogNextInput` _asbp_player_pawn (delegate `DialogNextInput_Event_0`))
        (add `PlayerPawn.DialogPrevInput` _asbp_player_pawn (delegate `DialogPrevInput_Event_0`))
        (`self.UpdateDialog`)
        (add `self.OnDialogEnd` (delegate `OnDialogEnd_Event_0`)))
      (:`CastFailed`
        (`KismetSystemLibrary.PrintString` "Cast to player pawn failed in BP_DialogSystem")))))

(event `OnDialogChanged_Event_0` :!signature `self.OnDialogChanged`
  (params (Dialog :type "Dialog Structure"))
  (`/Game/Blueprints/Widgets/WBP_DialogueUI.ChangeDialogueText` (`self.DialogBox`) Dialog_DialogText)
  (`/Game/Blueprints/Widgets/WBP_DialogueUI.Change Dialogue Portrait` (`self.DialogBox`) Dialog_CharacterImage))

(event `DialogNextInput_Event_0`
  (`self.ProgressDialog`)
  (`KismetSystemLibrary.PrintString` "sheeeeeeeeet works"))

(event `DialogPrevInput_Event_0`
  (`self.RegressDialog`))

(event `OnDialogEnd_Event_0`
  (bind _outactors (`GameplayStatics.GetAllActorsOfClass` "/Game/Blueprints/System/BP_LevelSelector.BP_LevelSelector_C"))
  (`/Game/Blueprints/System/BP_LevelSelector.LoadLevel` (`|GetArrayItem` _outactors))
  (bind _foundwidgets (`WidgetBlueprintLibrary.GetAllWidgetsOfClass` "/Game/Blueprints/Widgets/WBP_DialogueUI.WBP_DialogueUI_C"))
  (for _array_element _foundwidgets
    (`Widget.RemoveFromParent` _array_element)))

(fn `UserConstructionScript`)