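; BP_LevelSelector is a level exit actor that moves the game to another level when the PlayerPawn overlaps its Trigger or LoadLevel is called.
; A one-shot IsLoadingLevel guard starts the optional EndLevelTransition Level Sequence and waits for it to finish, or proceeds immediately if none is set.
; It then advances the grief stage in BP_GameInstance if WasGriefLevel is set, clears HasDied and calls ChangeLevel.
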(event `self.ReceiveActorBeginOverlap`
  (params (OtherActor :type "Actor Object Reference")))

(event `LoadLevel`
  (bind _endleveltransition (`self.EndLevelTransition`))
  (if (not (`self.bIsLoadingLevel`)) :!label _label
    (set `self.bIsLoadingLevel` true)
    (if (`KismetSystemLibrary.IsValidSoftObjectReference` (`|ConvertAsset` _endleveltransition))
      (bind (_outactor _returnvalue) (`LevelSequencePlayer.CreateLevelSequencePlayer` _endleveltransition (make `MovieSceneSequencePlaybackSettings` true)))
      (add `MovieSceneSequencePlayer.OnFinished` _returnvalue (delegate `On Finished Sequence`))
      (else
        (if (`self.WasGriefLevel`) :!label _label_2
          (bind _asbp_game_instance (cast `/Game/Blueprints/System/BP_GameInstance` (`GameplayStatics.GetGameInstance`)))
          (`/Game/Blueprints/System/BP_GameInstance.AddGriefStage` _asbp_game_instance))
        (bind _asbp_game_instance_2 (cast `/Game/Blueprints/System/BP_GameInstance` (`GameplayStatics.GetGameInstance`)))
        (set `/Game/Blueprints/System/BP_GameInstance.HasDied` false _asbp_game_instance_2)
        (`self.ChangeLevel`)))))

(event `On Finished Sequence`
  (goto _label_2))

(event `self.Trigger.OnComponentBeginOverlap`
  (params (OverlappedComponent :type "PrimitiveComponent Object Reference") (OtherActor :type "Actor Object Reference") (OtherComp :type "PrimitiveComponent Object Reference") (OtherBodyIndex :type Integer) (bFromSweep :type Boolean) (SweepResult :type "HitResult Structure (by ref)"))
  (cast `PlayerPawn` OtherActor)
  (goto _label))

(fn `UserConstructionScript`)